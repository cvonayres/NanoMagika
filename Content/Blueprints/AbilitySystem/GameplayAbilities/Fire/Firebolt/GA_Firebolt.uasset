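; Firebolt gameplay ability that fires a projectile toward the point under the player's mouse.
; On activation it takes mouse target data, turns the avatar toward that location through the combat interface and plays the firebolt montage.
; A montage gameplay event times the projectile spawn, and the ability ends after a short delay.
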(event Ability|EventActivateAbility
  (bind _datahandle (|TargetDataUnderMouse)
    (:ValidData
      (Variables|Default|SetProjectileTargetLocation (.Location (Collision|BreakHitResult (Ability|TargetData|GetHitResultfromTargetData _datahandle))))
      (bind _asecmcombat_interface (Utilities|Casting|CastToECMCombatInterface (Ability|GetAvatarActorfromActorInfo)))
      (Class|ECMCombatInterface|UpdateFacingTarget _asecmcombat_interface (Variables|Default|GetProjectileTargetLocation))
      (|PlayMontageandWaitProxy "None" "/Game/Assets/Characters/Aura/Animations/Abilities/AM_Firebolt.AM_Firebolt" 1.0 "None" true 1.0 0.0 false
        (:then
          ;[1 1 1] Wait for AnimNotifier with correct tag
          (Ability|Tasks|WaitGameplayEvent "(TagName=\"Event.Montage.Firebolt\")" 0
            (:EventReceived
              (Class|ECMProjectileSpell|SpawnProjectile (Variables|Default|GetProjectileTargetLocation))
              (Utilities|FlowControl|Delay 1.0)
              (Ability|EndAbility))))))))

(event Ability|EventOnEndAbility
  (params (bWasCancelled :type Boolean)))