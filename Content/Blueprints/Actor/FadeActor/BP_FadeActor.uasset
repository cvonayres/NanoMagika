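; Actor that fades its mesh out and back in, with fades triggered from the Player Camera Manager.
; Construction caches the original materials and builds dynamic instances from the fade material list, which are swapped onto the mesh on FadeOut.
; A timeline, reversed for fade-in, drives their "Fade" parameter.
; On finish, originals are restored if Fade reaches one, and both branches set the mesh to ignore the Visibility channel.
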(event EventFadein
  ;[1 1 1] Called from Player Camera Manager - BP
  (bind _fade (Timeline|Fading Reverse)
    (:Update
      (CallFunction|UpdateFadeParam _fade))
    (:Finished
      (CallFunction|FadeFinished _fade))))

(event EventFadeOut
  ;[1 1 1] Called from Player Camera Manager - BP
  (CallFunction|SetMaterialstoDynamicInstances)
  (bind _fade (Timeline|Fading Play)
    (:Update
      (CallFunction|UpdateFadeParam _fade))
    (:Finished
      (CallFunction|FadeFinished _fade))))

(fn ConstructionScript
  (Variables|Default|SetOriginalMaterials (Rendering|Material|GetMaterials (Variables|Default|GetMesh)))
  (Utilities|Array|Clear (Variables|Default|GetDynamicMaterials))
  (for _array_element (Variables|Default|GetFadeMaterialInstances)
    (bind _returnvalue (Rendering|Material|CreateDynamicMaterialInstance _array_element "None" "None" :!class /Script/Engine.KismetMaterialLibrary))
    (Utilities|Array|AddUnique (Variables|Default|GetDynamicMaterials) _returnvalue)))

(fn SetMaterialstoDynamicInstances
  (for (_array_element _array_index) (Variables|Default|GetDynamicMaterials)
    (Rendering|Material|SetMaterial (Variables|Default|GetMesh) _array_index _array_element)))

(fn ResetMaterials
  (for (_array_element _array_index) (Variables|Default|GetOriginalMaterials)
    (Rendering|Material|SetMaterial (Variables|Default|GetMesh) _array_index _array_element)))

(fn UpdateFadeParam
  (params (InputPin :type Float%20%28single-precision%29))
  (for _array_element (Variables|Default|GetDynamicMaterials)
    (Rendering|Material|SetScalarParameterValue _array_element "Fade" InputPin :!class /Script/Engine.MaterialInstanceDynamic)))

(fn FadeFinished
  (params (A :type Float%20%28double-precision%29))
  (bind _returnvalue (>= A 1.0))
  (if _returnvalue
    (CallFunction|ResetMaterials)
    (Collision|SetCollisionResponsetoChannel (Variables|Default|GetMesh) "ECC_Visibility" "ECR_Ignore")
    (elif (<= _returnvalue 0)
      (Collision|SetCollisionResponsetoChannel (Variables|Default|GetMesh) "ECC_Visibility" "ECR_Ignore"))))