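; Base enemy character Blueprint that supplies the dissolve effect and the motion warp facing target for enemies.
; The dissolve event plays a timeline from the start, feeding its track into a helper that sets the "Dissolve" scalar on the valid mesh and weapon dynamic material instances.
; A second event writes the given location to the "FacingTarget" Motion Warping target.
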(event EventStartDissolveTimeline
  (params (DynamicMaterialInstance :type Material%20Instance%20Dynamic%20Object%20Reference) (WeaponDynamicMaterialInstance :type Material%20Instance%20Dynamic%20Object%20Reference))
  (bind _dissolvetrack (Timeline|Timeline PlayFromStart)
    (:Update
      (CallFunction|NewFunction _dissolvetrack DynamicMaterialInstance WeaponDynamicMaterialInstance))))

(event EventUpdateFacingTarget
  (params (Target :type Vector%20%28by%20ref%29 :default "0, 0, 0"))
  (Class|MotionWarpingComponent|AddorUpdateWarpTargetfromLocation (Variables|Default|GetMotionWarping) "FacingTarget" Target))

(fn ConstructionScript)

(fn NewFunction
  (params (InputPin :type Float%20%28single-precision%29) (MeshDissolveInst :type Material%20Instance%20Dynamic%20Object%20Reference) (WeaponDissolveInst :type Material%20Instance%20Dynamic%20Object%20Reference))
  (Utilities|FlowControl|Sequence
    (:then_0
      (bind _meshdissolveinst (LocalVariables|GetMeshDissolveInst)
        (:then
          (Rendering|Material|SetScalarParameterValue _meshdissolveinst "Dissolve" InputPin :!class /Script/Engine.MaterialInstanceDynamic))
        (:else)))
    (:then_1
      (bind _weapondissolveinst (LocalVariables|GetWeaponDissolveInst)
        (:then
          (Rendering|Material|SetScalarParameterValue _weapondissolveinst "Dissolve" InputPin :!class /Script/Engine.MaterialInstanceDynamic))
        (:else)))))