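; BP_PCM is a player-side Blueprint, likely a camera manager, holding an unfinished draft of runtime camera setup for the ECM character.
; BeginPlay and the construction script are empty, so the setup chain never runs.
; That disconnected chain casts to the ECM controller and character, then adds a spring arm on the root and a camera.
; The camera is never attached, as the last steps clear the spring arm reference and attach it to itself.
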(event EventBeginPlay)

(fn ConstructionScript)