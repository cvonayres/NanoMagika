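; GA_Firebolt is the hero's Firebolt gameplay ability, which fires a projectile at the location under the mouse.
; On activation it commits cost and cooldown, gets mouse target data, and turns the avatar toward the hit location through the combat interface.
; It plays the Firebolt montage and spawns the projectile when the montage's gameplay event arrives.
; The ability ends when the montage completes, is interrupted or is cancelled.
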(event Ability|EventActivateAbility
  ;[1 1 1] Required for cost and cooldown
  (Ability|CommitAbility)
  (bind _datahandle (|TargetDataUnderMouse)
    (:ValidData
      (Variables|Default|SetProjectileTargetLocation (.Location (Collision|BreakHitResult (Ability|TargetData|GetHitResultfromTargetData _datahandle))))
      (bind _asecmcombat_interface (Utilities|Casting|CastToECMCombatInterface (Ability|GetAvatarActorfromActorInfo)))
      (Class|ECMCombatInterface|UpdateFacingTarget _asecmcombat_interface (Variables|Default|GetProjectileTargetLocation))
      (|PlayMontageandWaitProxy "None" "/Game/Assets/Characters/Aura/Animations/Abilities/AM_Firebolt.AM_Firebolt" 1.0 "None" false 1.0 0.0 false
        (:then
          ;[1 1 1] Wait for AnimNotifier with correct tag
          (Ability|Tasks|WaitGameplayEvent "(TagName=\"Event.Montage.Firebolt\")" 0
            (:EventReceived
              (Class|ECMProjectileAttack|SpawnProjectile (Variables|Default|GetProjectileTargetLocation)))))
        (:OnCompleted
          (Ability|EndAbility :!label _label))
        (:OnInterrupted
          (goto _label))
        (:OnCancelled
          (goto _label))))))